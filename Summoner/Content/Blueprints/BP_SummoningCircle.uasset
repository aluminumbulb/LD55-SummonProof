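; Summoning circle actor that calls alchemy objects (BP_AlchOb) to its location by a summon key.
; On BeginPlay it caches every BP_AlchOb in the level.
; AttemptSummon finds the object with the matching key and teleports it above the circle by a Z offset, or prints a message if none matches.
; If an object is already summoned, the next attempt returns it to its original location and clears it instead.
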(event Custom|AttemptSummon
  (params (SummonID :type String))
  ;[1 1 1] Seek out summonable object with requested key by iterating through all objects
  (Variables|Default|GetCurrObj
    (:then
      ;[1 1 1] Return Object to Original Location and Clear
      (Transformation|SetActorLocation (Variables|Default|GetCurrObj) (Variables|/Game/Blueprints/Actors/BP_AlchOb.BP_AlchOb_C|GetOriginalLocation (Variables|Default|GetCurrObj)) false false)
      (Variables|Default|SetCurrObj 0))
    (:else
      (bind _array_element (Utilities|Array|ForEachLoopwithBreak (Variables|Default|GetTPAbleObj) :!label _label)
        (:LoopBody
          (if (Utilities|Enum|Equal(Enum) SummonID (Variables|/Game/Blueprints/Actors/BP_AlchOb.BP_AlchOb_C|GetSummonKey _array_element))
            (Variables|Default|SetCurrObj _array_element)
            (goto _label Break)))
        (:Completed
          (bind _currobj (Variables|Default|GetCurrObj)
            (:then
              (Default|TPtoSummon _currobj (+ (Transformation|GetActorLocation) (Math|Vector|MakeVector 0.0 0.0 (Variables|Default|GetZOffset)))))
            (:else
              ;;[1 1 1] TODO: Expose to User
              (Development|PrintString "No summon found by that key"))))))))

(event EventBeginPlay
  (bind _outactors (Actor|GetAllActorsOfClass "/Game/Blueprints/Actors/BP_AlchOb.BP_AlchOb_C"))
  (Variables|Default|SetTPAbleObj _outactors))

(fn ConstructionScript)

(fn SummonObject)