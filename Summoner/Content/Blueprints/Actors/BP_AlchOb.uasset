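; Alchemy object actor that can be summoned by a sigil combination and can trigger a player win.
; On BeginPlay it stores its original location and concatenates the Org, Use and Dir values of SigilCombo into a SummonKey string.
; TPtoSummon moves it to a given location without sweep and calls PlayerWon when WinningMover is set.
; Hovering the cursor over its mesh only prints a debug string.
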(event OnBeginCursorOver(StaticMesh)
  (params (TouchedComponent :type Primitive%20Component%20Object%20Reference))
  (Development|PrintString "Hello"))

(event Custom|TPtoSummon
  (params (ToLoc :type Vector))
  (Transformation|SetActorLocation ToLoc false false)
  (if (Variables|Default|GetWinningMover)
    (Default|CallPlayerWon)))

(event Custom|ParseSigilInfo
  (bind _sigilcombo (Variables|Default|GetSigilCombo))
  ;[1 1 1] Process Sigil Info
  (bind _output_get (Variables|Default|SetSummonKey ""))
  (Variables|Default|SetSummonKey (Utilities|String|Append _output_get (Utilities|String|ToString(Integer) (Math|Conversions|ToInteger(Byte) (.org _sigilcombo))) (Utilities|String|ToString(Integer) (Math|Conversions|ToInteger(Byte) (.use _sigilcombo))) (Utilities|String|ToString(Integer) (Math|Conversions|ToInteger(Byte) (.dir _sigilcombo))))))

(event EventBeginPlay
  (Variables|Default|SetOriginalLocation (Transformation|GetActorLocation))
  (CallFunction|ParseSigilInfo))

(event Collision|EventActorBeginOverlap
  (params (OtherActor :type Actor%20Object%20Reference)))

(event EventTick
  (params (DeltaSeconds :type Float%20%28single-precision%29)))

(fn ConstructionScript)