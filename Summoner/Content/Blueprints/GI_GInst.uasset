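; Game instance Blueprint (GI_GInst) with helper functions for adding and removing UI widgets on screen.
; AddWidgetToScreen declines a widget already in the viewport, otherwise adds it, shows the given player's mouse cursor and returns the widget.
; RemoveWidgetFromScreen removes the widget from its parent and leaves the cursor setting untouched.
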(fn AddWidgettoScreen
  (params (WidToAdd :type User%20Widget%20Object%20Reference) (OwnPlayer :type Player%20Controller%20Object%20Reference))
  ;[1 1 1] Initial Check
  (if (UserInterface|Viewport|IsinViewport WidToAdd)
    (Development|PrintString "Declined Existing Widget")
    (else
      (UserInterface|Viewport|AddtoViewport WidToAdd 0)
      (Variables|/Script/Engine.PlayerController|SetbShowMouseCursor OwnPlayer true)
      (return WidToAdd))))

(fn RemoveWidgetfromScreen
  (params (WidToRemove :type User%20Widget%20Object%20Reference) (OwnPlayer :type Player%20Controller%20Object%20Reference))
  (Widget|RemovefromParent WidToRemove))